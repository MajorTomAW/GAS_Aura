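; BP_EnemyBase is an enemy base Blueprint that darkens its cel-shaded mesh when it is shadowed from the light source.
; BeginPlay creates dynamic instances of the mesh's materials and caches ShadowDarkness from the MPC_CelShader parameter collection.
; Every Tick, it finds BP_LightSource and line-traces from the mesh against the light's forward direction.
; A hit sets each material's Strength to ShadowDarkness; otherwise Strength is full.
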(event `self.ReceiveBeginPlay`
  (`parent.ReceiveBeginPlay`)
  (for _array_element (`MeshComponent.GetMaterials` (`self.Mesh`))
    (bind _returnvalue (`KismetMaterialLibrary.CreateDynamicMaterialInstance` _array_element (`KismetStringLibrary.Conv_StringToName` (`KismetSystemLibrary.GetObjectName` _array_element))))
    (`KismetArrayLibrary.Array_Add` (`self.DynMaterials`) _returnvalue))
  (bind _returnvalue_2 (`KismetMaterialLibrary.GetScalarParameterValue` "/Game/Materials/Params/MPC_CelShader.MPC_CelShader" "ShadowDarkness"))
  (set `self.ShadowDarkness` _returnvalue_2))

(event `self.ReceiveTick`
  (params (DeltaSeconds :type "Float (single-precision)"))
  (bind _returnvalue (`SceneComponent.K2_GetComponentLocation` (`self.Mesh`)))
  (`parent.ReceiveTick` DeltaSeconds)
  (bind _returnvalue_2 (`GameplayStatics.GetActorOfClass` "/Game/Blueprints/GameObjects/Light/BP_LightSource.BP_LightSource_C"))
  (`/Engine/EditorBlueprintResources/StandardMacros.IsValid` _returnvalue_2
    (:`Is Valid`
      (bind (_outhit _returnvalue_3) (`KismetSystemLibrary.LineTraceSingle` :`Start` _returnvalue :`End` (+ _returnvalue (* (`KismetMathLibrary.GetForwardVector` (`self.K2_GetActorRotation` _returnvalue_2)) -10000.0)) :`TraceChannel` "TraceTypeQuery1" :`DrawTime` 1.0))
      (for (_array_element _array_index) (`self.DynMaterials`)
        (`MaterialInstanceDynamic.SetScalarParameterValue` _array_element "Strength" (`KismetMathLibrary.SelectFloat` (`self.ShadowDarkness`) 1.0 _returnvalue_3))
        (`PrimitiveComponent.SetMaterial` (`self.Mesh`) _array_index _array_element)))))

(fn `UserConstructionScript`)