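; BP_LightSource is a light actor that sets the scene's directional light color and shares it with the cel shader.
; It applies its LightColor variable to DirectionalLight1 and writes the same color to the EnvColor vector in the MPC_CelShader material parameter collection.
; The logic runs in both the construction script and BeginPlay, so it applies in the editor and at runtime.
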(event `self.ReceiveBeginPlay`
  (bind _returnvalue (`KismetMathLibrary.Conv_ColorToLinearColor` (`self.LightColor`)))
  (`LightComponent.SetLightColor` (`self.DirectionalLight1`) _returnvalue true)
  (`KismetMaterialLibrary.SetVectorParameterValue` "/Game/Materials/Params/MPC_CelShader.MPC_CelShader" "EnvColor" _returnvalue))

(fn `UserConstructionScript`
  (bind _returnvalue (`KismetMathLibrary.Conv_ColorToLinearColor` (`self.LightColor`)))
  (`LightComponent.SetLightColor` (`self.DirectionalLight1`) _returnvalue true)
  (`KismetMaterialLibrary.SetVectorParameterValue` "/Game/Materials/Params/MPC_CelShader.MPC_CelShader" "EnvColor" _returnvalue))